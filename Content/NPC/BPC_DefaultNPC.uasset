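; Default NPC Blueprint for a restaurant customer that gets seated when clicked.
; Left and right click share one path, which runs only while the blackboard's InRestaurant flag is set.
; It sets HaveATable, then asks MyRestaurantManager for a free table sized to the customer's group.
; The table's tile position, scaled to world units, becomes the Direction blackboard vector, with no check that a table was found.
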(event EventBeginPlay)

(event Collision|EventActorBeginOverlap
  (params (OtherActor :type Actor%20Object%20Reference)))

(event EventTick
  (params (DeltaSeconds :type Float%20%28single-precision%29)))

(event EventOnRightClick
  (bind _returnvalue (AI|GetBlackboard 0))
  (if (ScalableFloat|GetValueasBool _returnvalue (Utilities|Name|MakeLiteralName "InRestaurant"))
    (AI|Components|Blackboard|SetValueasBool _returnvalue (Utilities|Name|MakeLiteralName "HaveATable") true)
    (bind _returnvalue_2 (Actor|GetActorOfClass "/Game/MyRestaurantManager.MyRestaurantManager_C"))
    (bind _returnvalue_3 (Class|RestaurantManager|GetFreeTable _returnvalue_2 (Utilities|Array|Length (.allcustomers (Utilities|Array|Get(acopy) (Variables|/Script/DwarfBar.RestaurantManager|GetGroupCustomers _returnvalue_2) (Variables|Default|GetIndexGroup))))))
    (AI|Components|Blackboard|SetValueasVector (AI|GetBlackboard 0) (Utilities|Name|MakeLiteralName "Direction") (Math|Vector|MakeVector (* (.x (.TilePosition (Utilities|Struct|BreakTableData _returnvalue_3))) 1e+02) (* (.y (.TilePosition (Utilities|Struct|BreakTableData _returnvalue_3))) 1e+02) 0.0))))

(event EventOnLeftClick
  (bind _returnvalue (AI|GetBlackboard 0))
  (if (ScalableFloat|GetValueasBool _returnvalue (Utilities|Name|MakeLiteralName "InRestaurant"))
    (AI|Components|Blackboard|SetValueasBool _returnvalue (Utilities|Name|MakeLiteralName "HaveATable") true)
    (bind _returnvalue_2 (Actor|GetActorOfClass "/Game/MyRestaurantManager.MyRestaurantManager_C"))
    (bind _returnvalue_3 (Class|RestaurantManager|GetFreeTable _returnvalue_2 (Utilities|Array|Length (.allcustomers (Utilities|Array|Get(acopy) (Variables|/Script/DwarfBar.RestaurantManager|GetGroupCustomers _returnvalue_2) (Variables|Default|GetIndexGroup))))))
    (AI|Components|Blackboard|SetValueasVector (AI|GetBlackboard 0) (Utilities|Name|MakeLiteralName "Direction") (Math|Vector|MakeVector (* (.x (.TilePosition (Utilities|Struct|BreakTableData _returnvalue_3))) 1e+02) (* (.y (.TilePosition (Utilities|Struct|BreakTableData _returnvalue_3))) 1e+02) 0.0))))

(fn ConstructionScript)